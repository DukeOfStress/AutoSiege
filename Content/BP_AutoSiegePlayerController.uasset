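; Player controller for an auto-battler that presents hero selection, shop and battle phases on the client.
; BeginPlay spawns the board, card zones, Bob and opponent portrait on remote clients only.
; Server callbacks update zones, portraits and UI, resetting card positions when buy, play or sell fails.
; Battle results become queued animation objects that Tick plays sequentially, calling ServerBattleFinished when the queue is empty during battle.
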(event `self.ReceiveBeginPlay`
  (`/Engine/EditorBlueprintResources/ActorMacros.Switch Has Authority`
    (:`Remote`
      (bind _returnvalue (`|SpawnActorFromClass` "/Game/BP_Board.BP_Board_C" (`KismetMathLibrary.MakeTransform` (0.0 0.0 0.0)) "Undefined" "OverrideRootScale" null null))
      (bind _output_get (set `self.PlayerBoard` _returnvalue))
      (`self.SetViewTargetWithBlend` _output_get)
      (bind _returnvalue_2 (`|SpawnActorFromClass` "/Game/BP_CardZone.BP_CardZone_C" (`KismetMathLibrary.MakeTransform` (0.0 -300.0 0.0)) "Undefined" "OverrideRootScale" null null))
      (bind _output_get_2 (set `self.OpponentCardZone` _returnvalue_2))
      (set `/Game/BP_CardZone.Type` "OpponentBoard" _output_get_2)
      (bind _returnvalue_3 (`|SpawnActorFromClass` "/Game/BP_CardZone.BP_CardZone_C" (`KismetMathLibrary.MakeTransform` (0.0 150.0 0.0)) "Undefined" "OverrideRootScale" null null))
      (bind _output_get_3 (set `self.PlayerBoardCardZone` _returnvalue_3))
      (set `/Game/BP_CardZone.Type` "PlayerBoard" _output_get_3)
      (bind _returnvalue_4 (`|SpawnActorFromClass` "/Game/BP_CardZone.BP_CardZone_C" (`KismetMathLibrary.MakeTransform` (0.0 1000.0 0.0)) "Undefined" "OverrideRootScale" null null))
      (bind _output_get_4 (set `self.PlayerHandCardZone` _returnvalue_4))
      (set `/Game/BP_CardZone.Type` "PlayerHand" _output_get_4)
      (bind _returnvalue_5 (`|SpawnActorFromClass` "/Game/BP_Bob.BP_Bob_C" (`KismetMathLibrary.MakeTransform` (0.0 -765.0 0.0) (struct) (5.0 5.0 5.0)) "Undefined" "OverrideRootScale" null null))
      (set `self.Bob` _returnvalue_5)
      (bind _returnvalue_6 (`|SpawnActorFromClass` "/Game/BP_Portrait.BP_Portrait_C" (`KismetMathLibrary.MakeTransform` (0.0 -765.0 0.0) (struct) (5.0 5.0 5.0)) "Undefined" "OverrideRootScale" null null))
      (bind _output_get_5 (set `self.OpponentPortrait` _returnvalue_6))
      (`self.SetActorHiddenInGame` _output_get_5 true)
      (`/Game/BP_Portrait.ToggleHealth` _output_get_5))))

(event `ResetCardLocation`
  (params (CardToReset :type "PlayerCard Structure") (CardZone :type "/Game/BP_CardZone Object Reference"))
  (bind (_value _returnvalue) (`BlueprintMapLibrary.Map_Find` (`/Game/BP_CardZone.Cards` CardZone) (`.UID` (break `PlayerCard` CardToReset))))
  (if _returnvalue
    (`self.K2_SetActorLocation` _value (`/Game/BP_Card.InitialLocation` _value) false false)))

(event `TransferCardToCardZone`
  (params (CardToTransfer :type "PlayerCard Structure") (FromCardZone :type "/Game/BP_CardZone Object Reference") (ToCardZone :type "/Game/BP_CardZone Object Reference"))
  (`/Game/BP_CardZone.AddPlayerCard` ToCardZone CardToTransfer)
  (`/Game/BP_CardZone.RemovePlayerCard` FromCardZone CardToTransfer)
  (`/Game/BP_CardZone.RefreshVisual` ToCardZone))

(event `HideBob`
  (`self.SetActorHiddenInGame` (`self.Bob`) true))

(event `ShowBob`
  (`self.SetActorHiddenInGame` (`self.Bob`) false))

(event `ShowOpponent`
  (params (Opponent :type "BattleOpponent Structure"))
  (bind (_id _hero _startinghealth) (break `BattleOpponent` Opponent))
  (bind _opponentportrait (`self.OpponentPortrait`))
  (bind _returnvalue (`|GetDataTableRow` "/Game/Data/Hero_DataTable.Hero_DataTable" _hero)
    (:`then`
      (`PrimitiveComponent.SetMaterial` (`/Game/BP_Portrait.Portrait` _opponentportrait) 1 (`.Material` (break `Hero` _returnvalue)))
      (`/Game/BP_Portrait.UpdateHealth` _opponentportrait _startinghealth false)
      (`self.SetActorHiddenInGame` _opponentportrait false))))

(event `HideOpponent`
  (`self.SetActorHiddenInGame` (`self.OpponentPortrait`) true))

(event `self.ReceiveTick`
  (params (DeltaSeconds :type "Float (single-precision)"))
  (bind _animationqueue (`self.AnimationQueue`))
  (bind _output (`|GetArrayItem` _animationqueue))
  (switch `GameStage` (`self.GameStage`)
    (:`Shop`
      _)
    (:`Battle`
      _))
  (if (> (`KismetArrayLibrary.Array_Length` _animationqueue) 0)
    (bind _isfinished (`/Game/Animations/IAnimation.Tick` _output DeltaSeconds))
    (if _isfinished
      (`KismetArrayLibrary.Array_RemoveItem` (`self.AnimationQueue`) _output))
    (else
      (switch `GameStage` (`self.GameStage`)
        (:`Battle`
          (`self.Server_BattleFinished`))))))

(event `self.BP_PresentHeroes`
  (params (Heroes :type "Array of Name (by ref)"))
  (for (_array_element _array_index) Heroes
    (bind _returnvalue (`|SpawnActorFromClass` "/Game/BP_Portrait.BP_Portrait_C" (`KismetMathLibrary.MakeTransform` (`KismetMathLibrary.MakeVector` (+ -400.0 (* _array_index 400.0)) 0.0 1000.0) (struct) (5.0 5.0 5.0)) "Undefined" "OverrideRootScale" null null))
    (`Portrait.ReceiveOnUpdatePortrait` _returnvalue _array_element)
    (`KismetArrayLibrary.Array_Add` (`self.HeroPortraits`) _returnvalue)))

(event `self.BP_HeroApproved`
  (params (HeroName :type Name) (Health :type Integer))
  (for _array_element (`self.HeroPortraits`)
    (if (== (`Portrait.CurrentHeroName` _array_element) HeroName)
      (bind _output_get (set `self.HeroPortrait` _array_element))
      (`/Game/BP_Portrait.UpdateHealth` _output_get Health false)
      (else
        (`self.K2_DestroyActor` _array_element)))))

(event `self.BP_AllPlayersReady`
  (params (Heroes :type "Array of Name (by ref)"))
  (bind _heroportrait (`self.HeroPortrait`))
  (bind _ui (`self.UI`))
  (bind _asauto_siege_hud (cast `AutoSiegeHUD` (`self.GetHUD`)))
  (bind _asbp_auto_siege_user_widget (cast `/Game/UI/BP_AutoSiegeUserWidget` (`AutoSiegeHUD.CurrentWidget` _asauto_siege_hud)))
  (bind _output_get (set `self.UI` _asbp_auto_siege_user_widget))
  (`/Game/BP_Board.ToggleDimmer` (`self.PlayerBoard`))
  (`/Game/UI/BP_AutoSiegeUserWidget.ShowHeroUI` _output_get)
  (`/Game/UI/BP_AutoSiegeUserWidget.ToggleLeaderboardUI` _output_get)
  (`/Game/UI/BP_AutoSiegeUserWidget.ToggleStartMessageUI` _output_get)
  (`self.K2_SetActorLocation` _heroportrait (0.0 615.0 0.0) false false)
  (`/Game/BP_Portrait.ToggleHealth` _heroportrait)
  (for (_array_element _array_index) Heroes
    (bind _returnvalue (`|GetDataTableRow` "/Game/Data/Hero_DataTable.Hero_DataTable" _array_element)
      (:`then`
        (bind _astexture_2d (cast `Texture2D` (`.Texture` (break `Hero` _returnvalue))))
        (switch `int` _array_index
          (:`0`
            (`Image.SetBrushFromTexture` (`/Game/UI/BP_AutoSiegeUserWidget.PortraitScore_0` _ui) _astexture_2d false))
          (:`1`
            (`Image.SetBrushFromTexture` (`/Game/UI/BP_AutoSiegeUserWidget.PortraitScore_1` _ui) _astexture_2d false))
          (:`2`
            (`Image.SetBrushFromTexture` (`/Game/UI/BP_AutoSiegeUserWidget.PortraitScore_2` _ui) _astexture_2d false))
          (:`3`
            (`Image.SetBrushFromTexture` (`/Game/UI/BP_AutoSiegeUserWidget.PortraitScore_3` _ui) _astexture_2d false))
          (:`4`
            (`Image.SetBrushFromTexture` (`/Game/UI/BP_AutoSiegeUserWidget.PortraitScore_5` _ui) _astexture_2d false))
          (:`5`
            (`Image.SetBrushFromTexture` (`/Game/UI/BP_AutoSiegeUserWidget.PortraitScore_4` _ui) _astexture_2d false))
          (:`6`
            (`Image.SetBrushFromTexture` (`/Game/UI/BP_AutoSiegeUserWidget.PortraitScore_6` _ui) _astexture_2d false))
          (:`7`
            (`Image.SetBrushFromTexture` (`/Game/UI/BP_AutoSiegeUserWidget.PortraitScore_7` _ui) _astexture_2d false)))))))

(event `self.BP_ShowBattle`
  (params (Opponent :type "BattleOpponent Structure") (Battle :type "Battle Structure"))
  (bind (_actions _isdraw _losingplayer _newlosingplayerhealth) (break `Battle` Battle))
  (bind _opponentcardzone (`self.OpponentCardZone`))
  (set `self.GameStage` "Battle")
  (`self.ShowOpponent` Opponent)
  (`self.HideBob`)
  (`/Game/UI/BP_AutoSiegeUserWidget.HideShopUI` (`self.UI`))
  (`/Game/BP_CardZone.ClearZone` _opponentcardzone)
  (for _array_element (`.Cards` (break `BattleOpponent` Opponent))
    (`/Game/BP_CardZone.AddPlayerCard` _opponentcardzone _array_element))
  (`/Game/BP_CardZone.RefreshVisual` _opponentcardzone)
  (bind _returnvalue (`|GenericCreateObject` "/Game/Animations/Splash_Animation.Splash_Animation_C" self))
  (`/Game/Animations/Splash_Animation.Initialize` _returnvalue 3.0 "NewEnumerator0" (`self.UI`))
  (`KismetArrayLibrary.Array_Add` (`self.AnimationQueue`) _returnvalue)
  (for _array_element_2 _actions
    (bind _asbp_auto_siege_player_state (cast `/Game/BP_AutoSiegePlayerState` (`self.PlayerState`)))
    (bind (_currentplayer _type _attackeruid _defenderuid _newattackerhealth _newdefenderhealth) (break `BattleAction` _array_element_2))
    (if (== (`AutoSiegePlayerState.PlayerIndex` _asbp_auto_siege_player_state) _currentplayer)
      (bind _returnvalue_2 (`|GenericCreateObject` "/Game/Animations/CardAttack_Animation.CardAttack_Animation_C" self))
      (`/Game/Animations/CardAttack_Animation.Initialize` _returnvalue_2 (`BlueprintMapLibrary.Map_Find` (`/Game/BP_CardZone.Cards` (`self.PlayerBoardCardZone`)) _attackeruid) (`BlueprintMapLibrary.Map_Find` (`/Game/BP_CardZone.Cards` (`self.OpponentCardZone`)) _defenderuid) 0 0 _newattackerhealth _newdefenderhealth)
      (`KismetArrayLibrary.Array_Add` (`self.AnimationQueue`) _returnvalue_2)
      (else
        (bind _returnvalue_3 (`|GenericCreateObject` "/Game/Animations/CardAttack_Animation.CardAttack_Animation_C" self))
        (`/Game/Animations/CardAttack_Animation.Initialize` _returnvalue_3 (`BlueprintMapLibrary.Map_Find` (`/Game/BP_CardZone.Cards` (`self.OpponentCardZone`)) _attackeruid) (`BlueprintMapLibrary.Map_Find` (`/Game/BP_CardZone.Cards` (`self.PlayerBoardCardZone`)) _defenderuid) 0 0 _newattackerhealth _newdefenderhealth)
        (`KismetArrayLibrary.Array_Add` (`self.AnimationQueue`) _returnvalue_3))))
  (if (not _isdraw)
    (bind _asbp_auto_siege_player_state_2 (cast `/Game/BP_AutoSiegePlayerState` (`self.PlayerState`)))
    (if (== _losingplayer (`AutoSiegePlayerState.PlayerIndex` _asbp_auto_siege_player_state_2))
      (bind _returnvalue_4 (`|GenericCreateObject` "/Game/Animations/HeroDamage_Animation.HeroDamage_Animation_C" self))
      (`/Game/Animations/HeroDamage_Animation.Initialize` _returnvalue_4 (`self.HeroPortrait`) _newlosingplayerhealth)
      (`KismetArrayLibrary.Array_Add` (`self.AnimationQueue`) _returnvalue_4)
      (else
        (bind _returnvalue_5 (`|GenericCreateObject` "/Game/Animations/HeroDamage_Animation.HeroDamage_Animation_C" self))
        (`/Game/Animations/HeroDamage_Animation.Initialize` _returnvalue_5 (`self.OpponentPortrait`) _newlosingplayerhealth)
        (`KismetArrayLibrary.Array_Add` (`self.AnimationQueue`) _returnvalue_5)))))

(event `self.BP_BuyCard`
  (params (Succeeded :type Boolean) (BoughtCard :type "PlayerCard Structure") (NewGold :type Integer))
  (if Succeeded
    (`/Game/UI/BP_AutoSiegeUserWidget.UpdateGold` (`self.UI`) NewGold false)
    (`self.TransferCardToCardZone` BoughtCard (`self.OpponentCardZone`) (`self.PlayerHandCardZone`))
    (else
      (`self.ResetCardLocation` BoughtCard (`self.OpponentCardZone`)))))

(event `self.BP_PlayCard`
  (params (Succeeded :type Boolean) (CardPlayed :type "PlayerCard Structure"))
  (if Succeeded
    (`self.TransferCardToCardZone` CardPlayed (`self.PlayerHandCardZone`) (`self.PlayerBoardCardZone`))
    (else
      (`self.ResetCardLocation` CardPlayed (`self.PlayerHandCardZone`)))))

(event `self.BP_SellCard`
  (params (Succeeded :type Boolean) (CardSold :type "PlayerCard Structure") (NewGold :type Integer))
  (if Succeeded
    (`/Game/UI/BP_AutoSiegeUserWidget.UpdateGold` (`self.UI`) NewGold false)
    (`/Game/BP_CardZone.RemovePlayerCard` (`self.PlayerBoardCardZone`) CardSold)
    (else
      (`self.ResetCardLocation` CardSold (`self.PlayerBoardCardZone`)))))

(event `self.BP_BeginShop`
  (params (Gold :type Integer) (PlayerCards :type "Array of PlayerCard Structure (by ref)") (NextOpponent :type Integer))
  (bind _ui (`self.UI`))
  (bind _opponentcardzone (`self.OpponentCardZone`))
  (`KismetSystemLibrary.PrintString` (`KismetStringLibrary.Conv_IntToString` NextOpponent))
  (bind _returnvalue (`|GenericCreateObject` "/Game/Animations/Splash_Animation.Splash_Animation_C" self))
  (`/Game/Animations/Splash_Animation.Initialize` _returnvalue 3.0 "NewEnumerator1" (`self.UI`))
  (`KismetArrayLibrary.Array_Add` (`self.AnimationQueue`) _returnvalue)
  (`/Game/UI/BP_AutoSiegeUserWidget.UpdateGold` _ui Gold true)
  (`/Game/UI/BP_AutoSiegeUserWidget.ShowShopUI` _ui)
  (`/Game/BP_CardZone.ClearZone` (`self.OpponentCardZone`))
  (`self.ShowBob`)
  (`self.HideOpponent`)
  (for _array_element PlayerCards
    (`/Game/BP_CardZone.AddPlayerCard` _opponentcardzone _array_element))
  (`/Game/BP_CardZone.RefreshVisual` _opponentcardzone)
  (set `self.GameStage` "Shop"))

(event `self.BP_UpgradeShopTier`
  (params (Succeeded :type Boolean) (NewShopTier :type Integer) (NewShopUpgradePrice :type Integer) (NewGold :type Integer))
  (bind _ui (`self.UI`))
  (if Succeeded
    (`/Game/UI/BP_AutoSiegeUserWidget.UpdateShopUpgradePrice` _ui NewShopUpgradePrice)
    (`/Game/UI/BP_AutoSiegeUserWidget.UpdateGold` _ui NewGold false)
    (`/Game/BP_Bob.UpgradeTier` (`self.Bob`) NewShopTier)
    (else
      (`KismetSystemLibrary.PrintString` "Failed to upgrade shop"))))

(event `self.BP_RefreshShop`
  (params (Succeeded :type Boolean) (NewCards :type "Array of PlayerCard Structure (by ref)") (NewGold :type Integer))
  (bind _opponentcardzone (`self.OpponentCardZone`))
  (if Succeeded
    (`/Game/BP_CardZone.ClearZone` _opponentcardzone)
    (`/Game/UI/BP_AutoSiegeUserWidget.UpdateGold` (`self.UI`) NewGold false)
    (for _array_element NewCards
      (`/Game/BP_CardZone.AddPlayerCard` _opponentcardzone _array_element))
    (`/Game/BP_CardZone.RefreshVisual` _opponentcardzone)
    (else
      (`KismetSystemLibrary.PrintString` "Failed to refresh shop"))))

(event `self.BP_ToggleFreezeShop`
  (params (IsShopFrozen :type Boolean))
  (`/Game/BP_CardZone.ToggleFreeze` (`self.OpponentCardZone`)))

(fn `UserConstructionScript`)