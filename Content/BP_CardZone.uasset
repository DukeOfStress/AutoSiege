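; BP_CardZone is a card zone actor that spawns and tracks player cards, with a toggleable mesh outline.
; AddPlayerCard spawns a BP_Card via CreateCard, appends the card data to Spots and maps the actor by UID in Cards.
; CreateCard fills material and text from a data table row keyed by BaseCardID, deriving tier from 512-wide ID blocks.
; Cards spawn at the zone's origin; AddPlayerCardAnimateZone is an empty stub.
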(event `ToggleZoneOutline`
  (`SceneComponent.SetVisibility` (`self.StaticMesh`) (not (`SceneComponent.bVisible` (`self.StaticMesh`))) false))

(event `AddPlayerCard`
  (params (NewCard :type "PlayerCard Structure"))
  (bind _card (`self.CreateCard` NewCard (`KismetMathLibrary.MakeTransform` (0.0 0.0 0.0))))
  (`KismetArrayLibrary.Array_Add` (`self.Spots`) NewCard)
  (`BlueprintMapLibrary.Map_Add` (`self.Cards`) (`.UID` (break `PlayerCard` NewCard)) _card))

(event `AddPlayerCardAnimateZone`)

(fn `CreateCard`
  (params (PlayerCard :type "PlayerCard Structure") (SpawnTransform :type "Transform Structure"))
  (returns (Card :type "/Game/BP_Card Object Reference"))
  (bind (_uid _basecardid) (break `PlayerCard` PlayerCard))
  (bind _returnvalue (`|GetDataTableRow` "/Game/Data/CardData_DataTable.CardData_DataTable" (`KismetStringLibrary.Conv_StringToName` (`KismetStringLibrary.Conv_IntToString` _basecardid)))
    (:`then`
      (bind _returnvalue_2 (`|SpawnActorFromClass` "/Game/BP_Card.BP_Card_C" (`KismetMathLibrary.MakeTransform` (+ (`self.K2_GetActorLocation`) (.location SpawnTransform)) (.rotation SpawnTransform) (.scale SpawnTransform)) "Undefined" "OverrideRootScale" null null))
      (bind (_name _power _health _material) (break `CardData` _returnvalue))
      (`PrimitiveComponent.SetMaterial` (`/Game/BP_Card.CardBase` _returnvalue_2) 1 _material)
      (`TextRenderComponent.K2_SetText` (`/Game/BP_Card.Name_Text` _returnvalue_2) (`KismetTextLibrary.Conv_NameToText` _name))
      (`TextRenderComponent.K2_SetText` (`/Game/BP_Card.Description_Text` _returnvalue_2) "")
      (`TextRenderComponent.K2_SetText` (`/Game/BP_Card.CardTier_Text` _returnvalue_2) (`KismetTextLibrary.Conv_IntToText` (+ (/ _basecardid 512) 1)))
      (`TextRenderComponent.K2_SetText` (`/Game/BP_Card.Attack_Text` _returnvalue_2) (`KismetTextLibrary.Conv_IntToText` _power))
      (`TextRenderComponent.K2_SetText` (`/Game/BP_Card.Health_Text` _returnvalue_2) (`KismetTextLibrary.Conv_IntToText` _health))
      (return _returnvalue_2))))

(fn `UserConstructionScript`)