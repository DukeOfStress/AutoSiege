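; BP_AutoSiegeGameStateBase is the game state Blueprint for AutoSiege, pushing replicated state changes to the local player's UI.
; OnRepHeroes and OnRepRoundTimer events each fetch the AutoSiegeHUD from player controller 0 and cast its CurrentWidget to AutoSiegeUserWidget.
; The widget then refreshes either the players-ready display or the round timer.
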(event `self.OnRep_Heroes`
  (bind _asauto_siege_hud (cast `AutoSiegeHUD` (`PlayerController.GetHUD` (`GameplayStatics.GetPlayerController` 0))))
  (bind _asauto_siege_user_widget (cast `/Game/UI/AutoSiegeUserWidget` (`AutoSiegeHUD.CurrentWidget` _asauto_siege_hud)))
  (`/Game/UI/AutoSiegeUserWidget.UpdatePlayersReady` _asauto_siege_user_widget))

(event `self.OnRep_RoundTimer`
  (bind _asauto_siege_hud (cast `AutoSiegeHUD` (`PlayerController.GetHUD` (`GameplayStatics.GetPlayerController` 0))))
  (bind _asauto_siege_user_widget (cast `/Game/UI/AutoSiegeUserWidget` (`AutoSiegeHUD.CurrentWidget` _asauto_siege_hud)))
  (`/Game/UI/AutoSiegeUserWidget.UpdateRoundTimer` _asauto_siege_user_widget))

(fn `UserConstructionScript`)