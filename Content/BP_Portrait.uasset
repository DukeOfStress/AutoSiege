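; BP_Portrait is a clickable hero portrait actor used for hero selection in the AutoSiege game.
; OnUpdatePortrait looks up a hero row in Hero_DataTable, stores the name and applies that hero's material to the portrait mesh.
; Clicking it tells the AutoSiege player controller to destroy the unused portraits and report the player ready to the server with the chosen hero.
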(event `self.Portrait.OnClicked`
  (params (TouchedComponent :type "PrimitiveComponent Object Reference") (ButtonPressed :type "Key Structure"))
  (bind _asbp_auto_siege_player_controller (cast `/Game/BP_AutoSiegePlayerController` (`GameplayStatics.GetPlayerController` 0)))
  (bind _asbp_portrait (cast `/Game/BP_Portrait` (`ActorComponent.GetOwner` TouchedComponent)))
  (`/Game/BP_AutoSiegePlayerController.DestroyUnusedHeroPortraits` _asbp_auto_siege_player_controller _asbp_portrait)
  (`AutoSiegePlayerController.Server_PlayerReady` _asbp_auto_siege_player_controller (`self.CurrentHeroName`)))

(event `self.ReceiveOnUpdatePortrait`
  (params (HeroName :type Name))
  (bind _returnvalue (`|GetDataTableRow` "/Game/Data/Hero_DataTable.Hero_DataTable" HeroName)
    (:`then`
      (set `self.CurrentHeroName` HeroName)
      (`PrimitiveComponent.SetMaterial` (`self.Portrait`) 1 (`.Material` (break `Hero` _returnvalue))))))

(fn `UserConstructionScript`)